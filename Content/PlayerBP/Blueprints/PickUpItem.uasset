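; Weapon pickup actor that gives ammo to the Player who overlaps it.
; BeginPlay polls until WeaponAsset is valid, applies it to the skeletal mesh, reapplies it five seconds later and starts a timed self-destruct.
; On overlap, it finds the player's weapon by matching mesh, adds BulletCount plus a fixed bonus to its total bullets, syncs CurrentWeapon if the names match, then destroys itself.
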(event `Destory self`
  (`self.K2_DestroyActor`))

(event `self.ReceiveBeginPlay`
  (if (not (`KismetSystemLibrary.IsValid` (`self.WeaponAsset`))) :!label _label
    (`KismetSystemLibrary.Delay` 0.1)
    (goto _label)
    (else
      (`SkinnedMeshComponent.SetSkinnedAssetAndUpdate` (`self.WeaponMesh`) (`self.WeaponAsset`) true)
      (`KismetSystemLibrary.K2_SetTimerDelegate` (delegate `Destory self`) 300.0)
      (`KismetSystemLibrary.Delay` 5.0)
      (`SkinnedMeshComponent.SetSkinnedAssetAndUpdate` (`self.WeaponMesh`) (`self.WeaponAsset`) true))))

(event `self.ReceiveActorBeginOverlap`
  (params (OtherActor :type "Actor Object Reference"))
  (`KismetSystemLibrary.PrintString` (`KismetSystemLibrary.GetDisplayName` OtherActor))
  (if (== (`GameplayStatics.GetObjectClass` OtherActor) "/Game/PlayerBP/Blueprints/Player.Player_C")
    (bind _asplayer (cast `/Game/PlayerBP/Blueprints/Player` OtherActor))
    (set `self.Player` _asplayer)
    (bind _weapons (`/Game/PlayerBP/Blueprints/Player.Weapons` _asplayer))
    (for (_array_element _array_index) _weapons
      (if (== (`.WeaponMesh_16_A01730FE98434A4BBF692B93C52D271B` (break `/Game/PlayerBP/Blueprints/WeaponStruct` _array_element)) (`self.WeaponAsset`))
        (break)))
    (bind _output_get (set `self.UpdatingWeapon` _array_element))
    (bind _structout (setmembers `/Game/PlayerBP/Blueprints/WeaponStruct` :`StructRef` _output_get :`TotalBulletCount` (+ (`.TotalBulletCount_7_5CB649B754496E19E9BE558C4FEE1944` (break `/Game/PlayerBP/Blueprints/WeaponStruct` (`self.UpdatingWeapon`))) (`self.BulletCount`) 4)))
    (`KismetArrayLibrary.Array_Set` _weapons _array_index _structout)
    (if (`KismetStringLibrary.EqualEqual_StrStr` (`.WeaponName_2_1DF7A3E9504C91A65ECF3BBA0F3F36ED` (break `/Game/PlayerBP/Blueprints/WeaponStruct` (`/Game/PlayerBP/Blueprints/Player.CurrentWeapon` (`self.Player`)))) (`.WeaponName_2_1DF7A3E9504C91A65ECF3BBA0F3F36ED` (break `/Game/PlayerBP/Blueprints/WeaponStruct` (`self.UpdatingWeapon`))))
      (set `/Game/PlayerBP/Blueprints/Player.CurrentWeapon` _structout (`self.Player`)))
    (`self.K2_DestroyActor`)))

(fn `UserConstructionScript`)